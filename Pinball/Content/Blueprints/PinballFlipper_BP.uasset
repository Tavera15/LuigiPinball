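; Pinball flipper Blueprint that swings its Flipper component through Flip and Flop events.
; Flip sets StartRotation to a mirrored angle based on the FlipperFacing side, then quickly rotates the component to it with MoveComponentTo.
; Flop rotates it to EndRotation over the same short time; its facing switch changes nothing, and EndRotation is never assigned in these graphs.
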(event EventBeginPlay)

(event Collision|EventActorBeginOverlap
  (params (OtherActor :type Actor%20Object%20Reference)))

(event EventTick
  (params (DeltaSeconds :type Float%20%28single-precision%29)))

(event EventFlip
  (switch Utilities|FlowControl|Switch|SwitchonFlipperType (Variables|Default|GetFlipperFacing)
    (:Left
      (Variables|Default|SetStartRotation "0,30.000000, 0"))
    (:Right
      (Variables|Default|SetStartRotation "0,-30.000000, 0")))
  (Components|MoveComponentTo (Variables|Default|GetFlipper) "0, 0, 0" (Variables|Default|GetStartRotation) false false 0.02 false))

(event EventFlop
  (switch Utilities|FlowControl|Switch|SwitchonFlipperType (Variables|Default|GetFlipperFacing)
    (:Left
      _)
    (:Right
      _))
  (Components|MoveComponentTo (Variables|Default|GetFlipper) "0, 0, 0" (Variables|Default|GetEndRotation) false false 0.02 false))

(fn ConstructionScript)
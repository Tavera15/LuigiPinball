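; Pinball bumper actor that adds score through the PinballGM game mode when another actor overlaps it.
; Every overlap restarts a timeline, whether or not the game mode cast succeeds.
; Its BumpAlpha curve drives both the downward offset of BumperMech and the emissive boost on the bumper top.
; The construction script creates the dynamic material instance on BumperMesh that enables this glow.
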(event EventBeginPlay)

(event Collision|EventActorBeginOverlap
  (params (OtherActor :type Actor%20Object%20Reference))
  (bind _aspinball_gm (Utilities|Casting|CastToPinballGM (Game|GetGameMode))
    (:then
      (Default|TrackScore _aspinball_gm 1e+01)
      (bind _bumpalpha (Timeline|Timeline_0 PlayFromStart)
        (:Update
          (Transformation|SetRelativeLocation (Variables|Default|GetBumperMech) (Math|Vector|Lerp(Vector) "0, 0, 0" "0, 0,-70.000000" _bumpalpha) false false)
          (Rendering|Material|SetScalarParameterValue (Variables|Default|GetBumperTopMid) "EmissiveBoost" (Math|Float|Lerp 0.0 2e+01 _bumpalpha) :!class /Script/Engine.MaterialInstanceDynamic))))
    (:CastFailed
      (Timeline|Timeline_0 PlayFromStart))))

(event EventTick
  (params (DeltaSeconds :type Float%20%28single-precision%29)))

(fn ConstructionScript
  (bind _returnvalue (Rendering|Material|CreateDynamicMaterialInstance (Variables|Default|GetBumperMesh) 1 0 "None" :!class /Script/Engine.PrimitiveComponent))
  (Variables|Default|SetBumperTopMid _returnvalue))
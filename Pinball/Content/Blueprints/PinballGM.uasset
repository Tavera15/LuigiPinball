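; Pinball game mode that tracks score with a multiplier and spins the camera as the score climbs.
; On BeginPlay it finds the Camera_BP actor and makes it the player's view target.
; Tick watches for the score passing a limit, raises that limit by a fixed step, and picks a random yaw offset.
; A timeline then lerps the camera toward that rotation, feeding each result back as the next start.
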(event Custom|FindMyCamera
  (bind _outactors (Actor|GetAllActorsOfClass "/Game/Blueprints/Camera_BP.Camera_BP_C"))
  (bind _output_get (Variables|Default|SetMainCamera (Utilities|Array|Get(acopy) _outactors)))
  (Game|Player|SetViewTargetwithBlend (Game|GetPlayerController 0) _output_get 0.0 "VTBlend_Linear" 0.0 false))

(event EventBeginPlay
  (CallFunction|FindMyCamera))

(event EventTick
  (params (DeltaSeconds :type Float%20%28single-precision%29))
  (if (> (Variables|Default|GetScore) (Variables|Default|GetScoreLimit))
    (Variables|Default|SetScoreLimit (+ (Variables|Default|GetScoreLimit) 5e+02))
    (Variables|Default|SetCamRotator (Transformation|GetActorRotation (Variables|Default|GetMainCamera)))
    (Variables|Default|SetDesiredRot (Math|Rotator|MakeRotator (.x (+ (Math|Vector|MakeVector (.roll (Variables|Default|GetCamRotator)) (.pitch (Variables|Default|GetCamRotator)) (.yaw (Variables|Default|GetCamRotator))) (Math|Vector|MakeVector 0.0 0.0 (Math|Random|RandomFloatinRange -3.6e+02 3.6e+02)))) (.y (+ (Math|Vector|MakeVector (.roll (Variables|Default|GetCamRotator)) (.pitch (Variables|Default|GetCamRotator)) (.yaw (Variables|Default|GetCamRotator))) (Math|Vector|MakeVector 0.0 0.0 (Math|Random|RandomFloatinRange -3.6e+02 3.6e+02)))) (.z (+ (Math|Vector|MakeVector (.roll (Variables|Default|GetCamRotator)) (.pitch (Variables|Default|GetCamRotator)) (.yaw (Variables|Default|GetCamRotator))) (Math|Vector|MakeVector 0.0 0.0 (Math|Random|RandomFloatinRange -3.6e+02 3.6e+02))))))
    (bind _aplha (Timeline|RotateCam PlayFromStart)
      (:Update
        (Transformation|SetActorRotation (Variables|Default|GetMainCamera) (Math|Rotator|Lerp(Rotator) (Variables|Default|GetCamRotator) (Variables|Default|GetDesiredRot) _aplha))
        (Variables|Default|SetCamRotator (Math|Rotator|Lerp(Rotator) (Variables|Default|GetCamRotator) (Variables|Default|GetDesiredRot) _aplha))))))

(fn ConstructionScript)

(fn TrackScore
  (params (PointsToAdd :type Float%20%28single-precision%29))
  (bind _output_get (Variables|Default|SetScore (+ (* PointsToAdd (Variables|Default|GetMultiplier)) (Variables|Default|GetScore))))
  (return _output_get))